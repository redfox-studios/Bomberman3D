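; Blueprint function library of UI and debug helpers for a Bomberman game.
; GetAndFormatMatchInfo casts the player and game states to build score, lives, remaining time and stage texts, returning fallback text if a cast fails.
; CastFailed prints and returns a formatted cast-error message.
; Two other helpers pick a random formatted gameplay tip and a random UI background texture from arrays, printing a message when the array is empty.
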(fn `CastFailed`
  (params (CastToWhatFailed :type String) (CastFromWhatFailed :type String))
  (returns (Message_String :type String) (Message_Text :type Text))
  (bind _result (`|FormatText` "Cast to {Object} failed! Source: {Source}" (`KismetTextLibrary.Conv_StringToText` CastToWhatFailed) (`|GenericToText` CastFromWhatFailed)))
  (bind _returnvalue (`KismetTextLibrary.Conv_TextToString` _result))
  (`KismetSystemLibrary.PrintString` null _returnvalue)
  (return _returnvalue _result))

(fn `GetAndFormatMatchInfo`
  (returns (Score :type Text) (Lives :type Text) (TimeRemaining :type Text) (CurrentStage :type Text))
  (`|ExecutionSequence`
    (:`then_0`
      (bind _asbomberman_player_state (cast `BombermanPlayerState` (`GameplayStatics.GetPlayerState` null))
        (:`CastFailed`
          ; If fails (it wont, but just in case)
          (`self.CastFailed` "BombermanPlayerState"))))
    (:`then_1`
      (bind _asbomberman_game_state (cast `BombermanGameState` (`GameplayStatics.GetGameState` null))
        (:`CastFailed`
          (`self.CastFailed` "BombermanGameState"))))
    (:`then_2`
      (return (`|FormatText` "Score: {0}" (`PlayerState.Score` _asbomberman_player_state)) (`|FormatText` "Lives: {0}" (`BombermanPlayerState.Lives` _asbomberman_player_state)) (`|FormatText` "Time remaining: {0}" (`BombermanGameState.StageTimeRemaining` _asbomberman_game_state)) (`|FormatText` "Stage: {0}" (`BombermanGameState.CurrentStage` _asbomberman_game_state)))))
  (return "Something Went Wrong" "Something Went Wrong" "Something Went Wrong" "Something Went Wrong"))

(fn `GetRandomBombermanTexture`
  (returns (RandomizedTexture :type "Texture Object Reference") (RandomizedTextureArrayIndex :type Integer))
  (locals (TextureArray :type "Array of Texture Object Reference") (ArrayIndex :type Integer))
  (bind _texturearray (`local.TextureArray`))
  (bind (_outitem _outindex) (`KismetArrayLibrary.Array_Random` _texturearray))
  (if (`KismetArrayLibrary.Array_IsEmpty` _texturearray)
    (`KismetSystemLibrary.PrintString` null "TextureArray is empty")
    (else
      (return _outitem _outindex))))

(fn `GetRandomTip`
  (returns (RandomizedTip :type String) (RandomizedTipIndex :type Integer) (FormattedTipText :type Text))
  (locals (GameTips :type "Array of String"))
  (bind _gametips (`local.GameTips`))
  (bind (_outitem _outindex) (`KismetArrayLibrary.Array_Random` _gametips))
  (if (`KismetArrayLibrary.Array_IsEmpty` _gametips)
    (`KismetSystemLibrary.PrintString` null "GameTips array is empty nigga")
    (else
      (return _outitem _outindex (`|FormatText` "Tip #{TipIndex}: {TipContent}" (`KismetTextLibrary.Conv_IntToText` _outindex) (`KismetTextLibrary.Conv_StringToText` _outitem))))))